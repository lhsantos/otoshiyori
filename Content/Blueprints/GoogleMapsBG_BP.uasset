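; Google Maps background Blueprint that refreshes its map texture around the latest reported position.
; Each position change is printed on screen as debug text, saved as the last position and sent through a DoOnce gate that requests a map centered there.
; When a map texture arrives, it is applied and the gate resets after a short delay, throttling requests to a minimum interval.
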(event `OnMapTextureReceived`
  (params (Texture :type "Texture2D Object Reference"))
  (`self.UpdateTexture` Texture)
  ;[1 1 1] Minimum 5s interval between requests
  (`KismetSystemLibrary.Delay` 5.0)
  (goto _label :!via `Reset`))

(event `OnPositionChanged`
  (params (Position :type "PositionData Structure (by ref)"))
  (bind (_position _altitude _accuracy) (break `PositionData` Position))
  (`KismetSystemLibrary.PrintString` (`KismetStringLibrary.Concat_StrStr` "Position: " (`KismetStringLibrary.Conv_Vector2dToString` _position) "; Altitude: " (`KismetStringLibrary.Conv_DoubleToString` _altitude) "; Accuracy: " (`KismetStringLibrary.Conv_DoubleToString` _accuracy)) true true (struct :`R` 1.0 :`A` 1.0) 20.0)
  (bind _output_get (set `self.LastPosition` Position))
  ;[1 1 1] Triggers a new texture request
  (`/Engine/EditorBlueprintResources/StandardMacros.DoOnce` false :!label _label
    (:`Completed`
      (`GoogleMapsComponent.RequestMap` (`self.GoogleMaps`) (`.Position` (break `PositionData` _output_get)) 0.0 (`|CreateDelegate` :!event `OnMapTextureReceived`)))))

(fn `UserConstructionScript`)